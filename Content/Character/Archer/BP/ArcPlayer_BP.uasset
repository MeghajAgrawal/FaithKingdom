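; Archer player character Blueprint that extends a parent class with an aiming camera zoom and equipped-weapon body rotation.
; Aiming runs separate timelines for zoom in and out, lerping camera field of view and the spring arm's sideways offset.
; Each tick while equipped, it snaps actor yaw to the control rotation past a threshold and messages control pitch and yaw to the anim instance, zeroing the blend when unequipped.
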(event `self.ReceiveActorBeginOverlap`
  (params (OtherActor :type "Actor Object Reference"))
  (`parent.ReceiveActorBeginOverlap` OtherActor))

(event `self.ReceiveTick`
  (params (DeltaSeconds :type "Float (single-precision)"))
  (bind (_returnvalue_roll _returnvalue_pitch _returnvalue_yaw) (`KismetMathLibrary.BreakRotator` (`self.GetControlRotation`)))
  (bind (_returnvalue_roll_2 _returnvalue_pitch_2 _returnvalue_yaw_2) (`KismetMathLibrary.BreakRotator` (`self.K2_GetActorRotation`)))
  (bind _returnvalue (`SkeletalMeshComponent.GetAnimInstance` (`self.Mesh`)))
  (`parent.ReceiveTick` DeltaSeconds)
  (if (`self.IsEquipped`)
    (if (> (`KismetMathLibrary.Abs` (- _returnvalue_yaw (select `bool` (> _returnvalue_yaw_2 0.0) :`false` (+ _returnvalue_yaw_2 360.0) :`true` _returnvalue_yaw_2))) 60.0)
      (`self.K2_SetActorRotation` (`KismetMathLibrary.MakeRotator` 0.0 0.0 _returnvalue_yaw)))
    (message `/Game/Blueprints/Interface/BPI_CharacterAnimation.UPRotation` _returnvalue 0.5 (`KismetMathLibrary.MakeRotator` 100.0 _returnvalue_pitch _returnvalue_yaw))
    (else
      (message `/Game/Blueprints/Interface/BPI_CharacterAnimation.UPRotation` _returnvalue 0.0 (struct)))))

(event `self.EnableAiming`
  (params (Aiming :type Boolean))
  (`parent.EnableAiming` Aiming)
  (if Aiming
    (bind (_direction _fieldofview _targetarmlength) (`Timeline|Timeline_0`)
      (:`Update`
        (`CameraComponent.SetFieldOfView` (`self.Camera`) (`KismetMathLibrary.Lerp` 90.0 45.0 _fieldofview))
        (set `SpringArmComponent.SocketOffset` (`KismetMathLibrary.MakeVector` 0.0 (`KismetMathLibrary.Lerp` 0.0 40.0 _targetarmlength)) (`self.SpringArm`))))
    (else
      (bind (_direction_2 _fieldofview_2 _targetarmlength_2) (`Timeline|Timeline_1` :!via `Reverse`)
        (:`Update`
          (`CameraComponent.SetFieldOfView` (`self.Camera`) (`KismetMathLibrary.Lerp` 90.0 45.0 _fieldofview_2))
          (set `SpringArmComponent.SocketOffset` (`KismetMathLibrary.MakeVector` 0.0 (`KismetMathLibrary.Lerp` 0.0 40.0 _targetarmlength_2)) (`self.SpringArm`)))))))

(fn `UserConstructionScript`
  (`parent.UserConstructionScript`))