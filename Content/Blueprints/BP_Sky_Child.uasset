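; BP_Sky_Child is a sky Blueprint child that runs a continuous day/night cycle.
; Tick advances Time by a fixed step per frame, so cycle speed depends on frame rate, then calls UpdateTime.
; UpdateTime maps Time on a 24-hour wrap to the directional light's pitch, flags a material refresh and calls UpdateSky.
; The construction script also runs UpdateTime before the parent's script.
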(event `self.ReceiveTick`
  (params (DeltaSeconds :type "Float (single-precision)"))
  (set `self.Time` (+ (`self.Time`) 0.0005))
  (`self.UpdateTime`))

(fn `UpdateTime`
  (`self.K2_SetActorRotation` (`self.Directional light actor`) (`KismetMathLibrary.MakeRotator` 0.0 (+ (* (/ (mod (`self.Time`) 24.0) 24.0) 360.0) 90.0)) false)
  (set `self.Refresh material` true)
  (`self.UpdateSky`))

(fn `UserConstructionScript`
  (`self.UpdateTime`)
  (`parent.UserConstructionScript`))