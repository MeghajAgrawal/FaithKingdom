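; Weather controller that runs a one-shot, timed sequence of clouds thickening, rain starting, then both easing off.
; On BeginPlay it attaches the rain particles to the player, then drives cloud targets and ToggleRain, which switches particles, background audio and rain level.
; Tick steps the sky's CloudOpacity and the RainLevel in MPC_GLobal toward their targets by a fixed per-frame ChangeRate with a deadband, then refreshes the clouds.
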(event `self.ReceiveBeginPlay`
  (`KismetSystemLibrary.Delay` 0.2)
  (`SceneComponent.K2_AttachToComponent` (`self.P_Rain`) (`Actor.RootComponent` (`GameplayStatics.GetPlayerCharacter` 0)) "None" "SnapToTarget" "SnapToTarget" "SnapToTarget" true)
  (`KismetSystemLibrary.Delay` 5.0)
  (set `self.TargetCloudOpacity` 7.0)
  (`KismetSystemLibrary.Delay` 10.0)
  (`self.ToggleRain` true)
  (`KismetSystemLibrary.Delay` 30.0)
  (`self.ToggleRain` false)
  (set `self.TargetCloudOpacity` 1.0))

(event `self.ReceiveTick`
  (params (DeltaSeconds :type "Float (single-precision)"))
  (bind _cloud_opacity (`/Engine/EngineSky/BP_Sky_Sphere.Cloud opacity` (`self.Sky`)))
  (bind _returnvalue (- (`self.TargetCloudOpacity`) _cloud_opacity))
  (if (> (`KismetMathLibrary.Abs` _returnvalue) 0.1)
    (set `/Engine/EngineSky/BP_Sky_Sphere.Cloud opacity` (+ _cloud_opacity (* (`self.ChangeRate`) (`KismetMathLibrary.SelectFloat` 1.0 -1.0 (> _returnvalue 0.1)))) (`self.Sky`)))
  (bind _returnvalue_2 (`KismetMaterialLibrary.GetScalarParameterValue` "/Game/Materials/MPC_GLobal.MPC_GLobal" "RainLevel"))
  (bind _returnvalue_3 (- (`self.RainLevel`) _returnvalue_2))
  (if (> (`KismetMathLibrary.Abs` _returnvalue_3) 0.1)
    (`KismetMaterialLibrary.SetScalarParameterValue` "/Game/Materials/MPC_GLobal.MPC_GLobal" "RainLevel" (+ _returnvalue_2 (* (`self.ChangeRate`) (`KismetMathLibrary.SelectFloat` 1.0 -1.0 (> _returnvalue_3 0.1))))))
  (`/Engine/EngineSky/BP_Sky_Sphere.UpdateCloud` (`self.Sky`)))

(event `ToggleRain`
  (params (enable :type Boolean))
  (if enable
    (`ActorComponent.Activate` (`self.P_Rain`) false)
    (`AudioComponent.Play` (`self.Rain_Background`) 0.0)
    (set `self.RainLevel` 0.9)
    (else
      (`ActorComponent.Deactivate` (`self.P_Rain`))
      (`AudioComponent.Stop` (`self.Rain_Background`))
      (set `self.RainLevel` 0.0))))

(fn `UserConstructionScript`)