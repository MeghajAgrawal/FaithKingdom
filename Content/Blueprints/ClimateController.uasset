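; Climate controller actor that endlessly cycles seasonal changes on a timed loop.
; BeginPlay loops through delays, setting targets for autumn, leaf fall, snow, spring and a season index; the spring target is only ever set to zero.
; Each Tick, the generic ParameterAutumn macro steps MPC_GLobal scalars toward their targets at fixed rates.
; Tick also lerps the season index, wrapped at four, into the Fading component's "Season" parameter.
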(event `self.ReceiveBeginPlay`
  (`KismetSystemLibrary.Delay` 5.0)
  (set `self.AutumnTransistion` 1.0 :!label _label)
  (set `self.targetSeasonValue` 1.0)
  (`KismetSystemLibrary.Delay` 20.0)
  (set `self.LeafFallTransistion` 5.0)
  (`KismetSystemLibrary.Delay` 1.0)
  (set `self.SnowTransistion` 4.0)
  (set `self.targetSeasonValue` 2.0)
  (set `self.AutumnTransistion` 0.0)
  (`KismetSystemLibrary.Delay` 20.0)
  (set `self.SnowTransistion` 0.0)
  (set `self.targetSeasonValue` 3.0)
  (set `self.SpringTransistion` 0.0)
  (set `self.LeafFallTransistion` 0.0)
  (`KismetSystemLibrary.Delay` 10.0)
  (set `self.CurrentSeason value` 0.0)
  (set `self.targetSeasonValue` 0.0)
  (set `self.SpringTransistion` 0.0)
  (`KismetSystemLibrary.Delay` 40.0)
  (goto _label))

(event `self.ReceiveTick`
  (params (DeltaSeconds :type "Float (single-precision)"))
  (`self.ParameterAutumn` "Autumn" (`self.AutumnTransistion`) 0.01
    (:`OutputPin`
      (`self.ParameterAutumn` "Snow Bias" (`self.SnowTransistion`) 0.01
        (:`OutputPin`
          (`self.ParameterAutumn` "Spring" (`self.SpringTransistion`)
            (:`OutputPin`
              (`self.ParameterAutumn` "LeavesFall" (`self.LeafFallTransistion`)
                (:`OutputPin`
                  (bind _output_get (set `self.CurrentSeason value` (mod (`KismetMathLibrary.Lerp` (`self.CurrentSeason value`) (`self.targetSeasonValue`) 0.05) 4.0)))
                  (`AudioComponent.SetFloatParameter` (`self.Fading`) "Season" _output_get))))))))))

(fn `UserConstructionScript`)